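; Openable door actor that swings open and shut when the OpenDoor_BP interface's OnOpen and OnClose events fire.
; The closed rotation is cached at BeginPlay, and a DoorSwing timeline adds its OpenAngle yaw to it each update.
; A Sound Timing event track plays the Doorlock sound at the door's location during the swing.
; Closing reverses the same timeline.
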(event `self.ReceiveBeginPlay`
  (set `self.initialRotation` (`self.K2_GetActorRotation`)))

(event `self.OpenDoor_BP.onOpen`
  (bind (_direction _open_angle) (`Timeline|Door Swing` :!label _label)
    (:`Update`
      (`self.K2_SetActorRotation` (`KismetMathLibrary.ComposeRotators` (`KismetMathLibrary.MakeRotator` 0.0 0.0 _open_angle) (`self.initialRotation`))))
    (:`Sound Timing`
      (`GameplayStatics.PlaySoundAtLocation` "/Game/Audio/door-lock.door-lock" (`self.K2_GetActorLocation`)))))

(event `self.OpenDoor_BP.onClose`
  (goto _label :!via `Reverse`))

(fn `UserConstructionScript`)